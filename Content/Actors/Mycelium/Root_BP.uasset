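; Mycelium root actor that draws itself as a chain of spline mesh segments along its Spline component.
; The MyceliumRender event steps along the spline by SectionLength, adding a Z-forward spline mesh component for each section.
; Each segment takes local start and end positions from the spline, with tangent lengths clamped to SectionLength.
; The construction script holds a disconnected copy of this loop, so segments are built only when MyceliumRender is called.
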(event `self.MyceliumRender`
  (bind _spline (`self.Spline`))
  (bind _spline_2 (`self.Spline`))
  (for _index (range (+ (`KismetMathLibrary.FTrunc` (/ (`SplineComponent.GetSplineLength` (`self.Spline`)) (`self.SectionLength`))) 1))
    (bind _returnvalue (`AddComponent|NODE_AddSplineMeshComponent-5`))
    (`SplineMeshComponent.SetForwardAxis` _returnvalue "Z" true)
    (bind _returnvalue_2 (* (`self.SectionLength`) _index))
    (bind _returnvalue_3 (* (`self.SectionLength`) (+ _index 1)))
    (`SplineMeshComponent.SetStartAndEnd` _returnvalue (`SplineComponent.GetLocationAtDistanceAlongSpline` _spline_2 _returnvalue_2 "Local") (`KismetMathLibrary.ClampVectorSize` (`SplineComponent.GetTangentAtDistanceAlongSpline` _spline_2 _returnvalue_2 "Local") 0.0 (`self.SectionLength`)) (`SplineComponent.GetLocationAtDistanceAlongSpline` _spline _returnvalue_3 "Local") (`KismetMathLibrary.ClampVectorSize` (`SplineComponent.GetTangentAtDistanceAlongSpline` _spline _returnvalue_3 "Local") 0.0 (`self.SectionLength`)) true)))

(fn `UserConstructionScript`)