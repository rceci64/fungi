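; Mycelium actor that lays a chain of spline meshes along an editable spline, with no active gameplay logic.
; The construction script splits the spline into sections whose length follows the actor's X scale, adding a Z-forward spline mesh component for each.
; Each segment takes its endpoints and tangents from the spline in local space, with tangents clamped to section length.
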(fn `UserConstructionScript`
  (bind _returnvalue_x (`KismetMathLibrary.BreakVector` (`self.GetActorScale3D`)))
  (bind _spline (`self.Spline`))
  (bind _spline_2 (`self.Spline`))
  (set `self.Section Length` (* 100.0 _returnvalue_x))
  (for _index (range (+ (`KismetMathLibrary.FTrunc` (/ (`SplineComponent.GetSplineLength` (`self.Spline`)) (`self.Section Length`))) 1))
    (bind _returnvalue (`AddComponent|NODE_AddSplineMeshComponent-0`))
    (`SplineMeshComponent.SetForwardAxis` _returnvalue "Z" true)
    (bind _returnvalue_2 (* (`self.Section Length`) _index))
    (bind _returnvalue_3 (* (`self.Section Length`) (+ _index 1)))
    (`SplineMeshComponent.SetStartAndEnd` _returnvalue (`SplineComponent.GetLocationAtDistanceAlongSpline` _spline_2 _returnvalue_2 "Local") (`KismetMathLibrary.ClampVectorSize` (`SplineComponent.GetTangentAtDistanceAlongSpline` _spline_2 _returnvalue_2 "Local") 0.0 (`self.Section Length`)) (`SplineComponent.GetLocationAtDistanceAlongSpline` _spline _returnvalue_3 "Local") (`KismetMathLibrary.ClampVectorSize` (`SplineComponent.GetTangentAtDistanceAlongSpline` _spline _returnvalue_3 "Local") 0.0 (`self.Section Length`)) true)))