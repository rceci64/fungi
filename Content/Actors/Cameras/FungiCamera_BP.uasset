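; FungiCamera is an orbit camera that centers on the level and becomes the first player's view target on BeginPlay.
; It derives its position from the LevelManager_BP width and height.
; While IsDragging is set, Tick yaws the spring arm by horizontal mouse movement scaled by DragSensibility.
; Disconnected legacy logic adjusts arm length by the share of Base_BP actors on screen, using IsInsideViewPort.
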(event `self.ReceiveBeginPlay`
  (bind _returnvalue (`GameplayStatics.GetActorOfClass` "/Game/Actors/Managers/LevelManager_BP.LevelManager_BP_C"))
  (`self.K2_SetActorLocation` self (`KismetMathLibrary.MakeVector` (+ (/ (* (`LevelManager.Width` _returnvalue) 100) 2.0) 25.0) (+ (/ (* (`LevelManager.Height` _returnvalue) 100) 2.0) 25.0) 50.0) false false)
  (`PlayerController.SetViewTargetWithBlend` (`GameplayStatics.GetPlayerController` 0) self 0.0 "VTBlend_EaseInOut" 0.0 false))

(event `self.ReceiveTick`
  (params (DeltaSeconds :type "Float (single-precision)"))
  (if (`self.bIsDragging`)
    (`SceneComponent.K2_AddRelativeRotation` (`self.SpringArm`) (`KismetMathLibrary.MakeRotator` 0.0 0.0 (* (`PlayerController.GetInputMouseDelta` (`GameplayStatics.GetPlayerController` 0)) (`self.DragSensibility`))) false false)))

(fn `IsInsideViewPort`
  (params (X :type "Float (double-precision)") (Y :type "Float (double-precision)"))
  (returns (ReturnValue :type Boolean))
  (bind (_returnvalue_x _returnvalue_y) (`KismetMathLibrary.BreakVector2D` (`WidgetLayoutLibrary.GetViewportSize`)))
  (return (not (or (< X 0.0) (< Y 0.0) (> X _returnvalue_x) (> Y _returnvalue_y)))))

(fn `UserConstructionScript`)