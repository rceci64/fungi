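; Player character Blueprint for Fungi that owns the pause and win menus and records level completion.
; On BeginPlay it creates both widgets collapsed in the viewport, and TogglePauseMenu shows or hides the pause menu.
; ShowWinScreen displays the step count and updates the save slot, using the numeric level name as index to mark completion, overwrite the best score unconditionally and unlock the next level.
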(event `self.ReceiveBeginPlay`
  (`self.AddUIWidgets`))

(event `self.TogglePauseMenu`
  (params (bPaused :type Boolean))
  (bind _pausemenu (`self.PauseMenu`))
  (if bPaused
    (`Widget.SetVisibility` _pausemenu "Visible")
    (else
      (`Widget.SetVisibility` _pausemenu "Collapsed"))))

(event `self.ShowWinScreen`
  (params (StepsToShow :type Integer))
  (bind _aswin_menu (cast `/Game/UI/WinMenu` (`self.WinMenu`)))
  (`/Game/UI/WinMenu.SetStepsNumber` _aswin_menu (`KismetStringLibrary.Conv_IntToString` StepsToShow))
  (bind _returnvalue (`GameplayStatics.GetCurrentLevelName` true))
  (bind _returnvalue_2 (`GameplayStatics.LoadGameFromSlot` "fungiSave"))
  (bind _asfungi_save_game (cast `/Game/Save/FungiSaveGame` _returnvalue_2))
  (bind _returnvalue_3 (`KismetStringLibrary.Conv_StringToInt` _returnvalue))
  (bind _returnvalue_4 (- _returnvalue_3 1))
  (`KismetArrayLibrary.Array_Set` (`/Game/Save/FungiSaveGame.isLevelCompleted` _asfungi_save_game) _returnvalue_4 true true)
  (`KismetArrayLibrary.Array_Set` (`/Game/Save/FungiSaveGame.bestLevelScore` _asfungi_save_game) _returnvalue_4 StepsToShow true)
  (`KismetArrayLibrary.Array_Set` (`/Game/Save/FungiSaveGame.isLevelUnlocked` _asfungi_save_game) _returnvalue_3 true true)
  (`GameplayStatics.SaveGameToSlot` _asfungi_save_game "fungiSave")
  (`Widget.SetVisibility` (`self.WinMenu`) "Visible"))

(fn `AddUIWidgets`
  (locals (NewLocalVar :type "/Game/UI/WinMenu Object Reference"))
  (bind _asplayer_controller (cast `PlayerController` (`self.GetController`)))
  (bind _returnvalue (`|CreateWidget` "/Game/UI/PauseMenu.PauseMenu_C" _asplayer_controller))
  (`UserWidget.AddToViewport` _returnvalue 0)
  (`Widget.SetVisibility` _returnvalue "Collapsed")
  (set `self.PauseMenu` _returnvalue)
  (bind _returnvalue_2 (`|CreateWidget` "/Game/UI/WinMenu.WinMenu_C"))
  (`UserWidget.AddToViewport` _returnvalue_2 0)
  (`Widget.SetVisibility` _returnvalue_2 "Collapsed")
  (set `self.WinMenu` _returnvalue_2))

(fn `UserConstructionScript`)