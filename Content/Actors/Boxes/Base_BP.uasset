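; Base grid tile actor with ground and plant meshes, randomly rotated and decorated on BeginPlay.
; Outside the main menu, it waits a random or origin-distance delay, then plays a sound and animates its cube's height on Tick from a curve.
; Timelines drive dynamic material parameters for funging and for highlighting scaled by correctness.
; UnFunge only clears the funged flag, leaving the material unchanged.
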(event `self.ReceiveBeginPlay`
  (`self.InitMesh`)
  (bind _returnvalue (`GameplayStatics.GetCurrentLevelName` true))
  (if (!= _returnvalue "MainMenuMap")
    (bind _returnvalue_2 (`GameplayStatics.GetActorOfClass` "/Game/Actors/Managers/LevelManager_BP.LevelManager_BP_C"))
    (switch `/Game/Animations/BlocksAnimation/AnimationSelector` (`self.SpawnAnimationType`)
      (:`NewEnumerator0`
        ;[1 1 1] Engage animation
        (`KismetSystemLibrary.Delay` (`KismetMathLibrary.RandomFloat`)))
      (:`NewEnumerator1`
        (`KismetSystemLibrary.Delay` (`KismetMathLibrary.MapRangeClamped` (`KismetMathLibrary.VSize2D` (`KismetMathLibrary.MakeVector2D` (`KismetMathLibrary.Conv_IntToDouble` (`self.GridX`)) (`KismetMathLibrary.Conv_IntToDouble` (`self.GridY`)))) 0.0 (`KismetMathLibrary.VSize2D` (`KismetMathLibrary.MakeVector2D` (`KismetMathLibrary.Conv_IntToDouble` (`LevelManager.Width` _returnvalue_2)) (`KismetMathLibrary.Conv_IntToDouble` (`LevelManager.Height` _returnvalue_2)))) 0.0 1.0))))
    (`GameplayStatics.PlaySound2D` "/Game/Sound/Cue_LevelStart.Cue_LevelStart" 1.0 1.0 0.0 null null)
    (set `self.ElapsedTime` 0.0)
    (set `self.bStartAnimation` true)))

(event `self.ReceiveTick`
  (params (DeltaSeconds :type "Float (single-precision)"))
  ;[1 1 1] Compute elapsed time
  (if (`self.bStartAnimation`)
    (if (>= DeltaSeconds 5.0)
      (set `self.bStartAnimation` false)
      (else
        (set `self.ElapsedTime` (+ (`self.ElapsedTime`) DeltaSeconds))
        (`self.AnimateEntry`)))))

(event `self.Funge`
  ;[1 1 1] Change material funged
  (set `self.bIsFunged` true)
  (bind (_direction _newtrack_0) (`Timeline|Timeline`)
    (:`Update`
      (`MaterialInstanceDynamic.SetScalarParameterValue` (`self.TerraMatInst`) "FungedValue" _newtrack_0))))

(event `self.UnFunge`
  ;[1 1 1] Change material funged
  (set `self.bIsFunged` false))

(event `self.DoHighlight`
  (params (Highlighted :type Boolean) (Correct :type Boolean))
  (bind _returnvalue (`KismetMathLibrary.Conv_BoolToDouble` Correct))
  (bind _terramatinst (`self.TerraMatInst`))
  (if Highlighted
    (bind (_direction _newtrack_0) (`Timeline|HighlightValueTimeline` :!label _label)
      (:`Update`
        (`MaterialInstanceDynamic.SetScalarParameterValue` _terramatinst "HightlightValue" (* _newtrack_0 (`KismetMathLibrary.MapRangeClamped` _returnvalue 0.0 1.0 0.6 1.0)))
        (`MaterialInstanceDynamic.SetScalarParameterValue` _terramatinst "CorrectValue" _returnvalue)
        (`MaterialInstanceDynamic.SetScalarParameterValue` (`self.GespaMatInst`) "HightlightValue" 0.0)
        (`MaterialInstanceDynamic.SetScalarParameterValue` (`self.GespaMatInst`) "CorrectValue" 1.0)))
    (else
      (goto _label :!via `Reverse`))))

(fn `AnimateEntry`
  (`SceneComponent.K2_SetRelativeLocation` (`self.Cube`) (`KismetMathLibrary.MakeVector` 0.0 0.0 (`KismetMathLibrary.MapRangeClamped` (`CurveFloat.GetFloatValue` (`self.Curve`) (`KismetMathLibrary.MapRangeClamped` (`self.ElapsedTime`) 0.0 (`self.AnimationTime`) 0.0 1.0)) 0.0 1.0 0.0 (`self.MaxHeightAnim`))) false false))

(fn `InitMesh`
  (bind _terra (`self.terra`))
  (bind _gespa (`self.gespa`))
  (bind _returnvalue (`PrimitiveComponent.CreateDynamicMaterialInstance` _terra 0 "/Game/Art/Terra/MAT_Terra_Inst.MAT_Terra_Inst" "None"))
  (bind _output_get (set `self.TerraMatInst` _returnvalue))
  (`PrimitiveComponent.SetMaterial` _terra 0 _output_get)
  (bind _returnvalue_2 (`PrimitiveComponent.CreateDynamicMaterialInstance` _gespa 0 "/Game/Art/Gespa/MAT_planta_inst.MAT_planta_inst" "None"))
  (bind _output_get_2 (set `self.GespaMatInst` _returnvalue_2))
  (`PrimitiveComponent.SetMaterial` _gespa 0 _output_get_2)
  (`self.Randomize`))

(fn `Randomize`
  (bind _output (`|GetArrayItem` (`self.Rotations`) (`KismetMathLibrary.RandomIntegerInRange` 0 3)))
  (`SceneComponent.K2_AddLocalRotation` (`self.terra`) (`KismetMathLibrary.MakeRotator` 0.0 0.0 _output) false false)
  (`SceneComponent.K2_AddLocalRotation` (`self.gespa`) (`KismetMathLibrary.MakeRotator` 0.0 0.0 _output) false false)
  (`SceneComponent.SetVisibility` (`self.cosa`) (and (`KismetMathLibrary.RandomBool`) (`KismetMathLibrary.RandomBool`)) false)
  (`SceneComponent.SetVisibility` (`self.cosa1`) (and (`KismetMathLibrary.RandomBool`) (`KismetMathLibrary.RandomBool`)) false)
  (`SceneComponent.SetVisibility` (`self.cosa2`) (and (`KismetMathLibrary.RandomBool`) (`KismetMathLibrary.RandomBool`)) false)
  (`SceneComponent.SetVisibility` (`self.floreta`) (and (`KismetMathLibrary.RandomBool`) (`KismetMathLibrary.RandomBool`) (`KismetMathLibrary.RandomBool`)) false)
  (`SceneComponent.SetVisibility` (`self.floreta1`) (and (`KismetMathLibrary.RandomBool`) (`KismetMathLibrary.RandomBool`) (`KismetMathLibrary.RandomBool`)) false))

(fn `UserConstructionScript`)