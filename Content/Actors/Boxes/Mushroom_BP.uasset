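; Mushroom actor Blueprint that randomizes its appearance when play begins.
; After the parent BeginPlay, it gives the Bolet mesh component a random static mesh from the BoletsMeshes array.
; It then sets a random, non-uniform world scale on that component, with a wider possible range on Z.
; Overlap and Tick events are disabled, and the construction script only calls the parent.
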(event `self.ReceiveBeginPlay`
  (bind _returnvalue (`KismetMathLibrary.RandomFloatInRange` 0.1 0.15))
  (bind _bolets_meshes (`self.bolets_meshes`))
  (bind _bolet (`self.bolet`))
  (`parent.ReceiveBeginPlay`)
  (`StaticMeshComponent.SetStaticMesh` _bolet (`|GetArrayItem` _bolets_meshes (`KismetMathLibrary.RandomIntegerInRange` 0 (- (`KismetArrayLibrary.Array_Length` _bolets_meshes) 1))))
  (`SceneComponent.SetWorldScale3D` _bolet (`KismetMathLibrary.MakeVector` _returnvalue _returnvalue (`KismetMathLibrary.RandomFloatInRange` 0.1 0.2))))

(fn `UserConstructionScript`
  (`parent.UserConstructionScript`))